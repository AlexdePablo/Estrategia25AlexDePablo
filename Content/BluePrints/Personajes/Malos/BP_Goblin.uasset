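; Goblin enemy for a strategy game that picks a target and goes after it on BeginPlay.
; Target choice reads GS_Estrategia, taking the first gold entry, else the first villager, else the town center.
; It binds to the target's AC_MainObjeto death event, issues AI MoveTo, and calls OnGetWork immediately rather than on arrival.
; Target death clears the working flag and reruns target search after a short delay.
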(event `self.ReceiveBeginPlay`
  (`parent.ReceiveBeginPlay`)
  (`self.EncontrarTarget`))

(event `EncontrarTarget`
  (bind _mtarget (`self.mTarget`))
  ;[0.01605 0.2292 0.08224] Encuentra al target y va a por el
  (`self.mTarget`
    (:`then`)
    (:`else`
      (`self.fGetTarget`)
      (bind _mtarget_2 (`self.mTarget`)
        (:`then`
          (add `/Game/BluePrints/ObjetoBasico/AC_MainObjeto.onDeath` (`self.GetComponentByClass` _mtarget_2 "/Game/BluePrints/ObjetoBasico/AC_MainObjeto.AC_MainObjeto_C") (delegate `OnTargetMuerto`))
          (`|AIMoveTo` self (`self.K2_GetActorLocation` _mtarget) _mtarget 10.0
            (:`then`
              (`self.OnGetWork` (`self.mTarget`) "NewEnumerator2"))))
        (:`else`)))))

(event `OnTargetMuerto`
  ;[0.03207 0.2127 0.401] Cuando muere el target busca otro
  (set `self.mWorking` false)
  (`KismetSystemLibrary.Delay` 0.2)
  (`self.EncontrarTarget`))

(fn `fGetTarget`
  (bind _asgs_estrategia (cast `/Game/BluePrints/GS_Estrategia` (`GameplayStatics.GetGameState`)))
  (bind _mposoros (`/Game/BluePrints/GS_Estrategia.mPosOros` _asgs_estrategia))
  (if (`KismetArrayLibrary.Array_IsValidIndex` _mposoros)
    (set `self.mTarget` (`|GetArrayItem` _mposoros))
    (else
      (bind _mposvillagers (`/Game/BluePrints/GS_Estrategia.mPosVillagers` _asgs_estrategia))
      (if (`KismetArrayLibrary.Array_IsValidIndex` _mposvillagers)
        (set `self.mTarget` (`|GetArrayItem` _mposvillagers))
        (else
          (set `self.mTarget` (`/Game/BluePrints/GS_Estrategia.mPosTC` _asgs_estrategia)))))))

(fn `UserConstructionScript`
  (`parent.UserConstructionScript`))