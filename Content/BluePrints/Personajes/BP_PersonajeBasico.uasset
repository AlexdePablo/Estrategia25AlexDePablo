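; Basic selectable character that shows a selection indicator when clicked and moves by AI to a given destination.
; On begin play it spawns its default controller, hides the Selection component and calls AddPossessable with the first player controller.
; A click reveals Selection and registers the character with that player controller through RegisterCharacterMessage.
; The Moveto event runs AIMoveTo and prints the destination for debugging.
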(event `self.ReceiveBeginPlay`
  (`|ExecutionSequence`
    (:`then_0`
      (`self.SpawnDefaultController`))
    (:`then_1`
      (`SceneComponent.SetHiddenInGame` (`self.Selection`) true false)
      (`MovieSceneSequenceExtensions.AddPossessable` null (`GameplayStatics.GetPlayerController` 0)))))

(event `self.ReceiveActorOnClicked`
  (params (ButtonPressed :type "Key Structure"))
  (`SceneComponent.SetHiddenInGame` (`self.Selection`) false false)
  (message `/Game/BluePrints/BPInterfaces/BPI_PlayerController.RegisterCharacter` (`GameplayStatics.GetPlayerController` 0) self))

(event `/Game/BluePrints/BPInterfaces/BPI_MoveCharacter.MoveTo`
  (params (Destination :type "Vector Structure"))
  (`|AIMoveTo` self Destination null
    (:`then`
      (`KismetSystemLibrary.PrintString` (`KismetStringLibrary.Conv_VectorToString` Destination)))))

(fn `UserConstructionScript`)