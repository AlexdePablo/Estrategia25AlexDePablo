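; Villager unit that takes work orders to gather resources or construct buildings, forwarding move commands to its parent class.
; OnGetWork stores the target and work type, then Repeat polls 2D distance until in range and stops movement.
; DoAction then loops on per-job delays, passing gathered resources to the player character or advancing construction through target interfaces.
; FBuild and FRecolect are stubs; the MoveToInteract and Recolect macros duplicate the approach polling.
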(event `self.ReceiveBeginPlay`
  (`parent.ReceiveBeginPlay`))

(event `/Game/BluePrints/BPInterfaces/BPI_MoveCharacter.MoveTo`
  (params (Destination :type "Vector Structure") (AcceptanceRadius :type "Float (double-precision)"))
  (`parent.MoveTo` Destination AcceptanceRadius))

(event `OnGetWork`
  (params (Actor :type "Actor Object Reference") (WorkType :type "/Game/BluePrints/Enums/EWorkType Enum" :default "NewEnumerator0"))
  (set `self.TargetActor` Actor)
  (set `self.mWorkType` WorkType)
  (`self.Repeat`))

(event `Repeat`
  (bind _output_get (set `self.mDistanceToObject` (`KismetMathLibrary.Vector_Distance2D` (`self.K2_GetActorLocation`) (`self.K2_GetActorLocation` (`self.TargetActor`)))))
  (set `self.mWorking` true)
  (if (and (> _output_get 50.0) (`self.mWorking`))
    (set `self.mDistanceToObject` (`KismetMathLibrary.Vector_Distance2D` (`self.K2_GetActorLocation`) (`self.K2_GetActorLocation` (`self.TargetActor`))))
    (`KismetSystemLibrary.Delay` 0.2)
    (`self.Repeat`)
    (else
      (`Controller.StopMovement` (`self.GetController`))
      (`self.DoAction`))))

(event `DoAction`
  (if (`self.mWorking`)
    (switch `/Game/BluePrints/Enums/EWorkType` (`self.mWorkType`)
      (:`NewEnumerator0`
        (bind _asbpi_recolectable (cast `/Game/BluePrints/BPInterfaces/BPI_Recolectable` (`self.TargetActor`)))
        (bind _resourcetype (`/Game/BluePrints/BPInterfaces/BPI_Recolectable.fRecolectResource` _asbpi_recolectable))
        (bind _asbp_player_character (cast `/Game/BluePrints/Player/BP_PlayerCharacter` (`GameplayStatics.GetPlayerCharacter` 0)))
        (`/Game/BluePrints/Player/BP_PlayerCharacter.fGetResource` _asbp_player_character _resourcetype)
        (`KismetSystemLibrary.Delay` (`self.mRecolectSpeed`))
        (`self.DoAction`))
      (:`NewEnumerator1`
        (bind _asbpi_edificable (cast `/Game/BluePrints/BPInterfaces/BPI_Edificable` (`self.TargetActor`)))
        (`/Game/BluePrints/BPInterfaces/BPI_Edificable.fEdifica` _asbpi_edificable)
        (`KismetSystemLibrary.Delay` (`self.mBuildSpeed`))
        (`self.DoAction`))
      (:`NewEnumerator3`
        (`KismetSystemLibrary.PrintString` "No Existeix")))))

(fn `fBuild`
  (`KismetSystemLibrary.PrintString` "Villager: Build"))

(fn `fRecolect`
  (params (ObjectPosition :type "Vector Structure"))
  (locals (distanceToObject :type "Float (double-precision)")))

(fn `UserConstructionScript`
  (`parent.UserConstructionScript`))