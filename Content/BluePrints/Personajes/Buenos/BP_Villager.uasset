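; Villager unit that gathers resources and constructs buildings, extending a parent character's movement and action logic.
; Recolect and Build call interfaces on the target actor, wait by their speed, then call DoAction again; gathered resources go to the player character.
; A spawn event passes the chosen actor to the player controller.
; MoveToInteract polls 2D distance and stops movement once near the location or no longer working.
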(event `self.ReceiveBeginPlay`
  (`parent.ReceiveBeginPlay`))

(event `/Game/BluePrints/BPInterfaces/BPI_MoveCharacter.MoveTo`
  (params (Destination :type "Vector Structure") (AcceptanceRadius :type "Float (double-precision)"))
  (`parent.MoveTo` Destination AcceptanceRadius))

(event `Recolect`
  (`KismetSystemLibrary.PrintString` "Recolect")
  (bind _asbpi_recolectable (cast `/Game/BluePrints/BPInterfaces/BPI_Recolectable` (`self.mTargetActor`)))
  (bind _resourcetype (`/Game/BluePrints/BPInterfaces/BPI_Recolectable.fRecolectResource` _asbpi_recolectable))
  (bind _asbp_player_character (cast `/Game/BluePrints/Player/BP_PlayerCharacter` (`GameplayStatics.GetPlayerCharacter` 0)))
  (`/Game/BluePrints/Player/BP_PlayerCharacter.fGetResource` _asbp_player_character _resourcetype)
  (`KismetSystemLibrary.Delay` (`self.mRecolectSpeed`))
  (`self.DoAction`))

(event `Build`
  (bind _asbpi_edificable (cast `/Game/BluePrints/BPInterfaces/BPI_Edificable` (`self.mTargetActor`)))
  (`/Game/BluePrints/BPInterfaces/BPI_Edificable.fEdifica` _asbpi_edificable)
  (`KismetSystemLibrary.Delay` (`self.mBuildSpeed`))
  (`self.DoAction`))

(event `/Game/BluePrints/BPInterfaces/BPI_CanSpawn.SpawnActorIntoTheWorldSI`
  (params (NewParam :type "Actor Class Reference"))
  (bind _asbp_player_controller (cast `/Game/BluePrints/Player/BP_PlayerController` (`GameplayStatics.GetPlayerController` 0)))
  (set `/Game/BluePrints/Player/BP_PlayerController.mActorToSPawn` NewParam _asbp_player_controller))

(fn `UserConstructionScript`
  (`parent.UserConstructionScript`))