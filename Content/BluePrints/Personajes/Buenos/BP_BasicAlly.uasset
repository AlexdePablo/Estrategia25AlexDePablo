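; Base Blueprint for allied units that take work orders, tinting the health bar widget blue on BeginPlay.
; OnGetWork stores a target and work type, then Repeat polls every 0.2 seconds until the unit overlaps any actor of the target's class.
; It then stops controller movement and DoAction switches on work type.
; Recolect and Build cast self to BP_Villager, a child-specific dependency, while Attack and None only print debug text.
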(event `self.ReceiveBeginPlay`
  (`parent.ReceiveBeginPlay`)
  (set `UserWidget.ColorAndOpacity` (struct :`B` 1.0 :`A` 1.0) (`WidgetComponent.GetWidget` (`self.HealthBarWidget`))))

(event `OnGetWork`
  (params (Actor :type "Actor Object Reference") (WorkType :type "/Game/BluePrints/Enums/EWorkType Enum" :default "NewEnumerator0"))
  (set `self.mTargetActor` Actor)
  (set `self.mWorkType` WorkType)
  (`self.Repeat`))

(event `Repeat`
  (bind _overlappingactors (`self.GetOverlappingActors` (`GameplayStatics.GetObjectClass` (`self.mTargetActor`))))
  (set `self.mWorking` true)
  (for _array_element _overlappingactors
    (`KismetSystemLibrary.PrintString` (`KismetSystemLibrary.GetDisplayName` _array_element)))
  (if (and (== (`KismetArrayLibrary.Array_Length` _overlappingactors) 0) (`self.mWorking`))
    (`KismetSystemLibrary.Delay` 0.2)
    (`self.Repeat`)
    (else
      (`Controller.StopMovement` (`self.GetController`))
      (`self.DoAction`))))

(event `DoAction`
  (if (`self.mWorking`)
    (switch `/Game/BluePrints/Enums/EWorkType` (`self.mWorkType`)
      (:`NewEnumerator0`
        (bind _asbp_villager (cast `/Game/BluePrints/Personajes/Buenos/BP_Villager` self))
        (`/Game/BluePrints/Personajes/Buenos/BP_Villager.Recolect` _asbp_villager))
      (:`NewEnumerator1`
        (bind _asbp_villager_2 (cast `/Game/BluePrints/Personajes/Buenos/BP_Villager` self))
        (`/Game/BluePrints/Personajes/Buenos/BP_Villager.Build` _asbp_villager_2))
      (:`NewEnumerator2`
        (`KismetSystemLibrary.PrintString` "ALATAQUEEEEE"))
      (:`NewEnumerator3`
        (`KismetSystemLibrary.PrintString` "No Existeix")))))

(fn `UserConstructionScript`
  (`parent.UserConstructionScript`))