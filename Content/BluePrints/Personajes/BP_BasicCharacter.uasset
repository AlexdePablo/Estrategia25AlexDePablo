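; Base selectable character, named BasicCharacter, that is clicked to select and moved by AI move orders.
; Construction loads range, attack, speed and defense stats from DT_Characters, keyed by the ACMainObjeto component's character name.
; Clicks register it with the player controller and show its Selection marker; Moveto runs AIMoveTo, then clears MWorking.
; FAttack only prints and CanBeSelected returns false, apparently as defaults.
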(event `self.ReceiveBeginPlay`
  (`|ExecutionSequence`
    (:`then_0`
      (`self.SpawnDefaultController`))
    (:`then_1`
      (`SceneComponent.SetHiddenInGame` (`self.Selection`) true false))
    (:`then_2`
      (set `CharacterMovementComponent.MaxWalkSpeed` (`self.mSpeed`) (`self.CharacterMovement`)))))

(event `/Game/BluePrints/BPInterfaces/BPI_MoveCharacter.MoveTo`
  (params (Destination :type "Vector Structure") (AcceptanceRadius :type "Float (double-precision)"))
  (`|AIMoveTo` self Destination null 10.0
    (:`then`
      (set `self.mWorking` false))))

(event `/Game/BluePrints/BPInterfaces/BPI_Selectable.ToggleSelect`
  (params (Selected :type Boolean))
  (`SceneComponent.SetHiddenInGame` (`self.Selection`) (not Selected) false))

(event `self.ReceiveActorOnClicked`
  (params (ButtonPressed :type "Key Structure"))
  (`KismetSystemLibrary.Delay` 0.1)
  (message `/Game/BluePrints/BPInterfaces/BPI_PlayerController.RegisterCharacter` (`GameplayStatics.GetPlayerController` 0) self)
  (`/Game/BluePrints/BPInterfaces/BPI_Selectable.ToggleSelect` true))

(fn `CanBeSelected`
  (returns (`Yes/No` :type Boolean))
  (return false))

(fn `fAttack`
  (`KismetSystemLibrary.PrintString` "BasicCharacter: Attack"))

(fn `UserConstructionScript`
  (`/Game/BluePrints/ObjetoBasico/AC_MainObjeto.fGetVariables` (`self.AC_MainObjeto`))
  (bind _returnvalue (`|GetDataTableRow` "/Game/BluePrints/Personajes/DT_Characters.DT_Characters" (`/Game/BluePrints/ObjetoBasico/AC_MainObjeto.CHARACTER_NAME` (`self.AC_MainObjeto`)))
    (:`then`
      (`|ExecutionSequence`
        (:`then_0`
          (bind (_mrange _mattackspeed _mattack _mspeed _mdefense) (break `/Game/BluePrints/Personajes/sCharacterInfo` _returnvalue))
          (set `self.mRange` _mrange))
        (:`then_1`
          (set `self.mAttackSpeed` _mattackspeed))
        (:`then_2`
          (set `self.mAttack` _mattack))
        (:`then_3`
          (set `self.mSpeed` _mspeed))
        (:`then_4`
          (set `self.mDefense` _mdefense))))))