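; BP_MundoCubos generates a flat grid world of blue, yellow and green cubes at BeginPlay, chosen by thresholding seeded noise.
; FPerlin averages 1D Perlin samples of X and Y and adds weighted octaves, though these reuse base coordinates, ignoring computed octave frequencies.
; BeginPlay averages both axis orders and prints each value.
; Unconnected graphs retain an earlier noise generator and a render-target pixel reading test.
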(event `self.ReceiveBeginPlay`
  (set `self.mSeed` (`KismetMathLibrary.RandomIntegerInRange` 0 10000))
  (for _index (range (+ (`self.mGridSize`) 1))
    (for _index_2 (range (+ (`self.mGridSize`) 1))
      (bind _sample (`self.fPerlin` _index _index_2))
      (bind _sample_2 (`self.fPerlin` _index_2 _index))
      (bind _returnvalue (/ (+ _sample_2 _sample) 2.0))
      (`KismetSystemLibrary.PrintString` (`KismetStringLibrary.Conv_DoubleToString` _returnvalue))
      (if (< _returnvalue 0.92)
        (bind _returnvalue_2 (`KismetMathLibrary.MakeTransform` (`KismetMathLibrary.MakeVector` (* _index 10.0) (* _index_2 10.0)) (struct) (0.1 0.1 0.1)))
        (`|SpawnActorFromClass` "/Game/BluePrints/BP_CubitoAzul.BP_CubitoAzul_C" _returnvalue_2 "Undefined" "MultiplyWithRoot" null null)
        (elif (> _returnvalue 1.1)
          (`|SpawnActorFromClass` "/Game/BluePrints/BP_CubitoVerde.BP_CubitoVerde_C" _returnvalue_2 "Undefined" "MultiplyWithRoot" null null)
          (else
            (`|SpawnActorFromClass` "/Game/BluePrints/BP_CubitoAmarillo.BP_CubitoAmarillo_C" _returnvalue_2 "Undefined" "MultiplyWithRoot" null null)))))))

(fn `fPerlin`
  (params (y :type Integer) (x :type Integer))
  (returns (Sample :type "Float (double-precision)"))
  (locals (xCoord :type "Float (double-precision)") (yCoord :type "Float (double-precision)") (sampleVariable :type "Float (double-precision)") (newFreq :type "Float (double-precision)") (xOctaveCoord :type "Float (double-precision)") (yOctaveCoord :type "Float (double-precision)") (octaveSample :type "Float (double-precision)"))
  (set `local.yCoord` (+ (`self.mSeed`) (* (/ y (`self.mScale`)) (`self.mFrequency`))))
  (set `local.xCoord` (+ (`self.mSeed`) (* (/ x (`self.mScale`)) (`self.mFrequency`))))
  (set `local.sampleVariable` (/ (+ (`KismetAnimationLibrary.K2_MakePerlinNoiseAndRemap` (`local.xCoord`) 0.0 1.0) (`KismetAnimationLibrary.K2_MakePerlinNoiseAndRemap` (`local.yCoord`) 0.0 1.0)) 2.0))
  (for _index (range 1 (+ (+ (`self.mOctaves`) 1) 1))
    (set `local.newFreq` (* (`self.mFrequency`) (* _index (`self.mLacunarity`))))
    (set `local.xOctaveCoord` (+ (`self.mSeed`) (* (`local.newFreq`) (/ x (`self.mScale`)))))
    (set `local.yOctaveCoord` (+ (`self.mSeed`) (* (`local.newFreq`) (/ y (`self.mScale`)))))
    (bind _output_get (set `local.octaveSample` (* (/ (+ (`KismetAnimationLibrary.K2_MakePerlinNoiseAndRemap` (`local.xCoord`) 0.0 1.0) (`KismetAnimationLibrary.K2_MakePerlinNoiseAndRemap` (`local.yCoord`) 0.0 1.0)) 2.0) (/ (`self.mPersistence`) _index))))
    (set `local.sampleVariable` (+ _output_get (`local.sampleVariable`))))
  (return (`local.sampleVariable`)))

(fn `UserConstructionScript`)