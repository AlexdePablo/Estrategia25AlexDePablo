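; RTS-style player controller for drag-box selection and orders to selected units.
; Selection projects screen-box corners onto the world and box-traces for pawns, keeping prior picks when Shift is held.
; RegisterCharacter also adds units, showing HUD info for a single selection.
; The action input sends units to the cursor hit with index-scaled acceptance radii, then assigns villager work or attacks based on the target's interfaces.
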(event `self.ReceiveBeginPlay`
  (`|ExecutionSequence`
    (:`then_0`
      (set `self.bShowMouseCursor` true))
    (:`then_1`
      (`EnhancedInputSubsystemInterface.AddMappingContext` (subsystem `EnhancedInputLocalPlayerSubsystem`) "/Game/BluePrints/Inputs/IMC_Base.IMC_Base" 0 (struct)))))

(event `EnhancedInput|/Game/BluePrints/Inputs/IA_Select`
  (params (ActionValue :type Boolean) (ElapsedSeconds :type "Float (double-precision)") (TriggeredSeconds :type "Float (double-precision)") (InputAction :type "InputAction Object Reference" :default "/Game/BluePrints/Inputs/IA_Select.IA_Select"))
  (bind (_locationx _locationy) (`self.GetMousePosition`))
  (bind (_deltax _deltay) (`self.GetInputMouseDelta`))
  (bind _selectedactors (`self.SelectedActors`))
  (:`Triggered`
    (if (or (!= _deltax 0.0) (!= _deltay 0.0))
      (bind _returnvalue (`WidgetLayoutLibrary.GetMousePositionOnViewport`))
      (message `/Game/BluePrints/BPInterfaces/BPI_Hud.fDrawSelectBox` (`self.GetHUD`) true (`self.MouseStartPos`) _returnvalue)))
  (:`Started`
    (bind _returnvalue_2 (`WidgetLayoutLibrary.GetMousePositionOnViewport`))
    (set `self.MouseStartPos` _returnvalue_2)
    (set `self.MouseStartSPos` (`KismetMathLibrary.MakeVector2D` _locationx _locationy)))
  (:`Completed`
    (message `/Game/BluePrints/BPInterfaces/BPI_Hud.fDrawSelectBox` (`self.GetHUD`) true (0.0 0.0) (0.0 0.0))
    (if (not (`|GetInputActionValue`))
      (for _array_element _selectedactors
        (message `/Game/BluePrints/BPInterfaces/BPI_Selectable.ToggleSelect` _array_element false)
        (bind _asbp_hud (cast `/Game/BluePrints/UI/BP_HUD` (`self.GetHUD`)))
        (`/Game/BluePrints/UI/BP_HUD.fGetInfoObject` :`self` _asbp_hud))
      (`KismetArrayLibrary.Array_Clear` _selectedactors))
    (`self.fSelectActors`)
    (`KismetSystemLibrary.PrintString` (`KismetStringLibrary.Conv_IntToString` (`KismetArrayLibrary.Array_Length` (`self.SelectedActors`))))))

(event `/Game/BluePrints/BPInterfaces/BPI_PlayerController.RegisterCharacter`
  (params (SelectedActor :type "Actor Object Reference"))
  (bind _returnvalue (`self.GetComponentByClass` (`|GetArrayItem` (`self.SelectedActors`)) "/Game/BluePrints/AC_MainObjeto.AC_MainObjeto_C"))
  (`KismetArrayLibrary.Array_AddUnique` (`self.SelectedActors`) SelectedActor)
  (if (== (`KismetArrayLibrary.Array_Length` (`self.SelectedActors`)) 1)
    (bind _asbp_hud (cast `/Game/BluePrints/UI/BP_HUD` (`self.GetHUD`)))
    (`/Game/BluePrints/UI/BP_HUD.fGetInfoObject` _asbp_hud true (make `/Game/BluePrints/Personajes/sObjectInfo` (`KismetStringLibrary.Conv_NameToString` (`/Game/BluePrints/AC_MainObjeto.CHARACTER_NAME` _returnvalue)) (`/Game/BluePrints/AC_MainObjeto.mCurrentHp` _returnvalue) (`/Game/BluePrints/AC_MainObjeto.mMaxHp` _returnvalue) (`/Game/BluePrints/AC_MainObjeto.mInfo` _returnvalue) (`/Game/BluePrints/AC_MainObjeto.mSprite` _returnvalue) (`/Game/BluePrints/AC_MainObjeto.mResourcesToBuild` _returnvalue)))
    (else
      (bind _asbp_hud_2 (cast `/Game/BluePrints/UI/BP_HUD` (`self.GetHUD`)))
      (`/Game/BluePrints/UI/BP_HUD.fGetInfoObject` :`self` _asbp_hud_2))))

(event `EnhancedInput|/Game/BluePrints/Inputs/IA_DoAction`
  (params (ActionValue :type Boolean) (ElapsedSeconds :type "Float (double-precision)") (TriggeredSeconds :type "Float (double-precision)") (InputAction :type "InputAction Object Reference" :default "/Game/BluePrints/Inputs/IA_DoAction.IA_DoAction"))
  (bind (_hitresult _returnvalue) (`self.GetHitResultUnderCursorByChannel` "TraceTypeQuery1"))
  (bind (_bblockinghit _binitialoverlap _time _distance _location _impactpoint _normal _impactnormal _physmat _hitactor) (`GameplayStatics.BreakHitResult` _hitresult))
  (:`Triggered`
    ;[1 1 1] Mirar la posicion mientras esta pulsado
    (if _returnvalue
      (set `self.CachedDestination` _location)
      (set `self.mActorInteractable` _hitactor)))
  (:`Completed`
    (`self.fMoveTo` (`self.CachedDestination`))
    (bind _mactorinteractable (`self.mActorInteractable`)
      (:`then`
        (`|ExecutionSequence`
          (:`then_0`
            (cast `/Game/BluePrints/BPInterfaces/BPI_Interactable` _mactorinteractable))
          (:`then_1`
            (cast `/Game/BluePrints/BPInterfaces/BPI_Recolectable` _mactorinteractable)
            (for _array_element (`self.SelectedActors`)
              (bind _asbp_villager (cast `/Game/BluePrints/Personajes/BP_Villager` _array_element))
              (`/Game/BluePrints/Personajes/BP_Villager.OnGetWork` _asbp_villager (`self.mActorInteractable`) "NewEnumerator0")))
          (:`then_2`
            (cast `/Game/BluePrints/BPInterfaces/BPI_Edificable` _mactorinteractable)
            (for _array_element_2 (`self.SelectedActors`)
              (bind _asbp_villager_2 (cast `/Game/BluePrints/Personajes/BP_Villager` _array_element_2))
              (`/Game/BluePrints/Personajes/BP_Villager.OnGetWork` _asbp_villager_2 (`self.mActorInteractable`) "NewEnumerator1")))
          (:`then_3`
            (cast `/Game/BluePrints/BPInterfaces/BPI_Damageable` _mactorinteractable)
            (for _array_element_3 (`self.SelectedActors`)
              (bind _asbp_basic_character (cast `/Game/BluePrints/Personajes/BP_BasicCharacter` _array_element_3))
              (`/Game/BluePrints/Personajes/BP_BasicCharacter.fAttack` _asbp_basic_character)))))
      (:`else`))))

(fn `fMoveTo`
  (params (Destination :type "Vector Structure"))
  (for (_array_element _array_index) (`self.SelectedActors`)
    (message `/Game/BluePrints/BPInterfaces/BPI_MoveCharacter.MoveTo` _array_element Destination (`KismetMathLibrary.Conv_IntToDouble` (* (+ _array_index 1) 1000)))))

(fn `fScreenToLandMapping`
  (params (ScreenPosition :type "Vector2D Structure (by ref)"))
  (returns (Location :type "Vector Structure"))
  (bind (_worldposition _worlddirection) (`GameplayStatics.DeprojectScreenToWorld` (`GameplayStatics.GetPlayerController` 0) ScreenPosition))
  (bind (_outhit _returnvalue) (`KismetSystemLibrary.LineTraceSingle` _worldposition (+ _worldposition (* _worlddirection 1000000.0)) "TraceTypeQuery1"))
  (if _returnvalue
    (return (`.Location` (`GameplayStatics.BreakHitResult` _outhit)))
    (else
      (return (0.0 0.0 0.0)))))

(fn `fSelectActors`
  (locals (MouseEndSPos :type "Vector2D Structure") (E1 :type "Vector Structure") (E2 :type "Vector Structure") (E3 :type "Vector Structure") (E4 :type "Vector Structure") (Actors :type "Array of Actor Object Reference"))
  (bind (_locationx _locationy) (`self.GetMousePosition`))
  (bind _array (`|MakeArray` "ObjectTypeQuery3" :!type "EObjectTypeQuery Enum"))
  (bind (_mouseendspos_x _mouseendspos_y) (`KismetMathLibrary.BreakVector2D` (`local.MouseEndSPos`)))
  (bind (_mousestartspos_x _mousestartspos_y) (`KismetMathLibrary.BreakVector2D` (`self.MouseStartSPos`)))
  (bind _returnvalue (`KismetMathLibrary.FMin` _mousestartspos_y _mouseendspos_y))
  (bind _returnvalue_2 (`KismetMathLibrary.FMin` _mousestartspos_x _mouseendspos_x))
  (bind _returnvalue_3 (`KismetMathLibrary.FMax` _mousestartspos_y _mouseendspos_y))
  (bind _returnvalue_4 (`KismetMathLibrary.FMax` _mousestartspos_x _mouseendspos_x))
  (bind _output_get (set `local.MouseEndSPos` (`KismetMathLibrary.MakeVector2D` _locationx _locationy)))
  (if (> (`KismetMathLibrary.Distance2D` _output_get (`self.MouseStartSPos`)) 1.0)
    (bind _output_get_2 (set `local.E1` (`self.fScreenToLandMapping` (`KismetMathLibrary.MakeVector2D` _returnvalue_2 _returnvalue))))
    (bind _output_get_3 (set `local.E2` (`self.fScreenToLandMapping` (`KismetMathLibrary.MakeVector2D` _returnvalue_4 _returnvalue))))
    (bind _output_get_4 (set `local.E3` (`self.fScreenToLandMapping` (`KismetMathLibrary.MakeVector2D` _returnvalue_4 _returnvalue_3))))
    (bind _output_get_5 (set `local.E4` (`self.fScreenToLandMapping` (`KismetMathLibrary.MakeVector2D` _returnvalue_2 _returnvalue_3))))
    (bind _returnvalue_5 (`KismetMathLibrary.VLerp` _output_get_2 _output_get_5 0.5))
    (bind _returnvalue_6 (- _output_get_4 _output_get_5))
    (bind _returnvalue_7 (`KismetMathLibrary.MakeVector` (* (`KismetMathLibrary.FMin` (`KismetMathLibrary.Vector_Distance` _output_get_2 _output_get_5) (`KismetMathLibrary.Vector_Distance` _output_get_3 _output_get_4)) 0.5) 10.0 400.0))
    (bind (_outhits _returnvalue_8) (`KismetSystemLibrary.BoxTraceMultiForObjects` _returnvalue_5 (+ _returnvalue_5 _returnvalue_6) _returnvalue_7 (`KismetMathLibrary.FindLookAtRotation` _output_get_2 _output_get_5) _array))
    (if _returnvalue_8
      (for _array_element _outhits
        (`KismetArrayLibrary.Array_AddUnique` (`local.Actors`) (`.HitActor` (`GameplayStatics.BreakHitResult` _array_element)))))
    (bind _returnvalue_9 (`KismetMathLibrary.VLerp` _output_get_3 _output_get_4 0.5))
    (bind (_outhits_2 _returnvalue_10) (`KismetSystemLibrary.BoxTraceMultiForObjects` _returnvalue_9 (- _returnvalue_9 _returnvalue_6) _returnvalue_7 (`KismetMathLibrary.FindLookAtRotation` _output_get_3 _output_get_4) _array))
    (if _returnvalue_10
      (for _array_element_2 _outhits_2
        (`KismetArrayLibrary.Array_AddUnique` (`local.Actors`) (`.HitActor` (`GameplayStatics.BreakHitResult` _array_element_2)))))
    (for _array_element_3 (`local.Actors`)
      (message `/Game/BluePrints/BPInterfaces/BPI_Selectable.ToggleSelect` _array_element_3 true)
      (`KismetArrayLibrary.Array_AddUnique` (`self.SelectedActors`) _array_element_3))))

(fn `UserConstructionScript`)