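; BP_TerrainGenerator builds a blocky heightmap terrain from BP_Cubito actors at BeginPlay.
; It loops over a configurable grid, offsets sample coordinates by a random seed, and spawns one scaled-down cube per cell at a stepped height.
; Despite its name, fOwnPerlin averages a sine and cosine wave rather than computing Perlin noise.
; The multi-octave noise function is an unused stub, and each cell also adds an unconfigured static mesh component.
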(event `self.ReceiveBeginPlay`
  (set `self.mSeed` (`KismetMathLibrary.RandomFloatInRange` 0.0 100000.0))
  (for _index (range (`self.mGridSizeX`))
    (for _index_2 (range (`self.mGridSizeY`))
      (bind _mhigh (`self.fOwnPerlin` (+ (* _index (`self.mPerlinScale`)) (`self.mSeed`)) (+ (* _index_2 (`self.mPerlinScale`)) (`self.mSeed`))))
      (`AddComponent|NODE_AddStaticMeshComponent-0`)
      (`|SpawnActorFromClass` "/Game/BluePrints/BP_Cubito.BP_Cubito_C" (`KismetMathLibrary.MakeTransform` (`KismetMathLibrary.MakeVector` (* _index 10.0) (* _index_2 10.0) (* (`KismetMathLibrary.FTrunc` (* (/ (+ _mhigh 1.0) 2.0) (`self.mHeightMultiplier`))) 10.0)) (struct) (0.1 0.1 0.1)) "Undefined" "MultiplyWithRoot" null null))))

(fn `fMultiOctavePerlinNoise2D`
  (params (PosX :type "Float (double-precision)") (PosY :type "Float (double-precision)"))
  (locals (Total :type "Float (double-precision)") (MaxValue :type "Float (double-precision)") (Frequency :type "Float (double-precision)") (Amplitude :type "Float (double-precision)"))
  (for _ (range (`self.Octaves`))
    _))

(fn `fOwnPerlin`
  (params (mPosX :type "Float (double-precision)") (mPosY :type "Float (double-precision)"))
  (returns (mHigh :type "Float (double-precision)"))
  (locals (mFrequency :type "Float (double-precision)" :default 10.0))
  (return (/ (+ (`KismetMathLibrary.DegSin` (* mPosX (`local.mFrequency`))) (`KismetMathLibrary.DegCos` (* mPosY (`local.mFrequency`)))) 2.0)))

(fn `UserConstructionScript`)