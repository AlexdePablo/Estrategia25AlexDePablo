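; Base building actor that can be constructed over time, using its hit points as build progress.
; The construction script loads variables through ACMainObjeto and reads the initial built state from the DT_Buildings row matching its name.
; Each FEdifica call adds a construction amount to HP until the maximum is reached, then marks it built.
; A blue widget health bar updates every tick, and clicks register the building with the player controller after a short delay.
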(event `self.ReceiveBeginPlay`
  (`/Game/BluePrints/UI/CharactersHP/UW_HealthBar.SetFillColor` (cast `/Game/BluePrints/UI/CharactersHP/UW_HealthBar` (`WidgetComponent.GetWidget` (`self.HealthBarWidget`)) :!pure true) (struct :`B` 1.0 :`A` 1.0)))

(event `/Game/BluePrints/BPInterfaces/BPI_Edificable.fEdifica`
  (if (>= (`/Game/BluePrints/ObjetoBasico/AC_MainObjeto.mCurrentHp` (`self.AC_MainObjeto`)) (`/Game/BluePrints/ObjetoBasico/AC_MainObjeto.mMaxHp` (`self.AC_MainObjeto`)))
    ;[1 0 0.766] Cuando el edificio es constuirdo
    (set `/Game/BluePrints/ObjetoBasico/AC_MainObjeto.mCurrentHp` (`/Game/BluePrints/ObjetoBasico/AC_MainObjeto.mMaxHp` (`self.AC_MainObjeto`)) (`self.AC_MainObjeto`))
    (if (not (`self.mBuilded`))
      (set `self.mBuilded` true)
      (`KismetSystemLibrary.PrintString` "Construido"))
    (else
      ;[1 0 0.0296] Construir Edificio
      (set `/Game/BluePrints/ObjetoBasico/AC_MainObjeto.mCurrentHp` (+ (`/Game/BluePrints/ObjetoBasico/AC_MainObjeto.mCurrentHp` (`self.AC_MainObjeto`)) (`self.mConstructionAmount`)) (`self.AC_MainObjeto`)))))

(event `self.ReceiveActorOnClicked`
  (params (ButtonPressed :type "Key Structure"))
  (`KismetSystemLibrary.Delay` 0.2)
  (message `/Game/BluePrints/BPInterfaces/BPI_PlayerController.RegisterCharacter` (`GameplayStatics.GetPlayerController` 0) self))

(event `self.ReceiveTick`
  (params (DeltaSeconds :type "Float (single-precision)"))
  (bind _asuw_health_bar (cast `/Game/BluePrints/UI/CharactersHP/UW_HealthBar` (`WidgetComponent.GetWidget` (`self.HealthBarWidget`))))
  (`ProgressBar.SetPercent` (`/Game/BluePrints/UI/CharactersHP/UW_HealthBar.mHealthBar` _asuw_health_bar) (/ (`/Game/BluePrints/ObjetoBasico/AC_MainObjeto.mCurrentHp` (`self.AC_MainObjeto`)) (`/Game/BluePrints/ObjetoBasico/AC_MainObjeto.mMaxHp` (`self.AC_MainObjeto`)))))

(fn `UserConstructionScript`
  (`/Game/BluePrints/ObjetoBasico/AC_MainObjeto.fGetVariables` (`self.AC_MainObjeto`))
  (bind _returnvalue (`|GetDataTableRow` "/Game/BluePrints/Mundo/Buildings/DT_Buildings.DT_Buildings" (`/Game/BluePrints/ObjetoBasico/AC_MainObjeto.CHARACTER_NAME` (`self.AC_MainObjeto`)))
    (:`then`
      (`|ExecutionSequence`
        (:`then_0`
          (set `self.mBuilded` (`.mBuilded_1_385CFEB5496C37B10454C5B84ECC1EDF` (break `/Game/BluePrints/Mundo/Buildings/sBuildInfo` _returnvalue))))))))