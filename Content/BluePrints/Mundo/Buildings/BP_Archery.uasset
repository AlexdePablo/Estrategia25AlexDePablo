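; BP_Archery is an archery building actor that can spawn actors of a given class into the world.
; Its SpawnActorIntotheWorld event takes the class and spawns it above the building's location with a small random horizontal offset and reduced scale.
; Spawns always succeed, adjusting position to avoid collisions where possible.
; BeginPlay, overlap and Tick are disabled stubs, and the construction script only calls the parent.
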(event `/Game/BluePrints/BPInterfaces/BPI_SpawnActor.SpawnActorIntoTheWorld`
  (params (NewParam :type "Actor Class Reference"))
  (`|SpawnActorFromClass` NewParam (`KismetMathLibrary.MakeTransform` (+ (`self.K2_GetActorLocation`) (`KismetMathLibrary.MakeVector` (`KismetMathLibrary.RandomFloatInRange` 0.0 10.0) (`KismetMathLibrary.RandomFloatInRange` 0.0 10.0) 100.0)) (struct) (0.3 0.3 0.3)) "AdjustIfPossibleButAlwaysSpawn" "MultiplyWithRoot" null null))

(fn `UserConstructionScript`
  (`parent.UserConstructionScript`))