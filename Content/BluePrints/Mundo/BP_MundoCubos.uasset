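; Generates the cube world at BeginPlay from a random seed, then has cube actors instance their lists and triggers player and enemy spawning.
; A delay-based loop macro dispatches one row at a time.
; Each cell averages two 1D Perlin samples, one per axis, to queue a transform on the low, medium or high cube actor.
; FPerlin sums weighted octaves, but each resamples the base coordinate, leaving OctaveCoord unused.
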(event Custom|CustomEvent
  (params (NewParam :type Integer))
  (for _index (range 0 (Variables|Default|GetmGridSize))
    (bind _sample (CallFunction|FPerlin NewParam))
    (bind _sample_2 (CallFunction|FPerlin _index))
    (Development|PrintString (Utilities|String|ToString(Float) (/ (+ _sample_2 _sample) 2.0)))
    (if (< (/ (+ _sample_2 _sample) 2.0) 0.5)
      (bind _returnvalue (Actor|GetActorOfClass "/Game/BluePrints/Mundo/Cubitos/BP_CubitoBajo.BP_CubitoBajo_C"))
      (Default|FAddCubetoList _returnvalue (Math|Transform|MakeTransform (Math|Vector|MakeVector (* NewParam 1e+01) (* _index 1e+01) 0.0) "0, 0, 0" "0.010000,0.010000,0.100000"))
      (elif (> (/ (+ _sample_2 _sample) 2.0) 0.8)
        (bind _returnvalue_2 (Actor|GetActorOfClass "/Game/BluePrints/Mundo/Cubitos/BP_CubitoAlto.BP_CubitoAlto_C"))
        (Default|FAddCubetoList _returnvalue_2 (Math|Transform|MakeTransform (Math|Vector|MakeVector (* NewParam 1e+01) (* _index 1e+01) 0.0) "0, 0, 0" "0.010000,0.010000,0.100000"))
        (else
          (bind _returnvalue_3 (Actor|GetActorOfClass "/Game/BluePrints/Mundo/Cubitos/BP_CubitoMedio.BP_CubitoMedio_C"))
          (Default|FAddCubetoList _returnvalue_3 (Math|Transform|MakeTransform (Math|Vector|MakeVector (* NewParam 1e+01) (* _index 1e+01) 0.0) "0, 0, 0" "0.010000,0.010000,0.100000")))))))

(event EventBeginPlay
  (EventDispatchers|BindEventtoInstantiateRow (delegate Custom|CustomEvent))
  (Variables|Default|SetmSeed (Math|Random|RandomIntegerinRange 0 10000))
  (bind _index (Utilities|ForChulo 0 (Variables|Default|GetmGridSize) 0.0)
    (:OutExec
      (Default|CallInstantiateRow _index))
    (:Completed
      (bind _returnvalue (Actor|GetActorOfClass "/Game/BluePrints/Mundo/Cubitos/BP_CubitoBajo.BP_CubitoBajo_C"))
      (Default|FInstanceCubes _returnvalue)
      (bind _returnvalue_2 (Actor|GetActorOfClass "/Game/BluePrints/Mundo/Cubitos/BP_CubitoMedio.BP_CubitoMedio_C"))
      (Default|FInstanceCubes _returnvalue_2)
      (bind _returnvalue_3 (Actor|GetActorOfClass "/Game/BluePrints/Mundo/Cubitos/BP_CubitoAlto.BP_CubitoAlto_C"))
      (Default|FInstanceCubes _returnvalue_3)
      (bind _returnvalue_4 (Actor|GetActorOfClass "/Game/BluePrints/Mundo/BP_SpawnerResources.BP_SpawnerResources_C"))
      (Default|FSpawnPlayer _returnvalue_4)
      (bind _asgs_estrategia (Utilities|Casting|CastToGS_Estrategia (Game|GetGameState)))
      (Default|SpawnEnemies _asgs_estrategia))))

(fn ConstructionScript)

(fn FPerlin
  (params (Coordenada :type Integer))
  (LocalVariables|SetCoord (|(((y/Scale)*Frequency)+Seed) Coordenada (Variables|Default|GetmScale) (Variables|Default|GetmFrequency) (Variables|Default|GetmSeed)))
  (LocalVariables|SetsampleVariable (Class|KismetAnimationLibrary|MakePerlinNoiseandRemap (LocalVariables|GetCoord) 0.0 1.0))
  (for _index (range 1 (+ (Variables|Default|GetmOctaves) 1))
    (LocalVariables|SetnewFreq (|((i*Lacunarity)*Frequency) _index (Variables|Default|GetmLacunarity) (Variables|Default|GetmFrequency)))
    (LocalVariables|SetOctaveCoord (|(((y/Scale)*Freq)+Seed) Coordenada (Variables|Default|GetmScale) (LocalVariables|GetnewFreq) (Variables|Default|GetmSeed)))
    (bind _output_get (LocalVariables|SetoctaveSample (|(x*(Persistence/Octave)) (Class|KismetAnimationLibrary|MakePerlinNoiseandRemap (LocalVariables|GetCoord) 0.0 1.0) (Variables|Default|GetmPersistence) _index)))
    (LocalVariables|SetsampleVariable (|(OcatveSample+variableSample) _output_get (LocalVariables|GetsampleVariable))))
  (return (LocalVariables|GetsampleVariable)))