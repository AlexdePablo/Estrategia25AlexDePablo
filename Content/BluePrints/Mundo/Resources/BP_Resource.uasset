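; BP_Resource is a clickable world resource actor that exposes its resource type.
; Its construction script calls FGetVariables on the ACMainObjeto component, and FRecolectResource returns the ResourceType.
; A click waits briefly, then passes the actor to the first player controller through RegisterCharacterMessage.
; FInteract is empty, and a HUD info-display call is left unwired.
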(event `self.ReceiveBeginPlay`)

(event `/Game/BluePrints/BPInterfaces/BPI_Interactable.fInteract`)

(event `self.ReceiveActorOnClicked`
  (params (ButtonPressed :type "Key Structure"))
  (`KismetSystemLibrary.Delay` 0.2)
  (message `/Game/BluePrints/BPInterfaces/BPI_PlayerController.RegisterCharacter` (`GameplayStatics.GetPlayerController` 0) self))

(fn `fRecolectResource`
  (returns (ResourceType :type "/Game/BluePrints/Enums/EResourceType Enum"))
  (return (`self.ResourceType`)))

(fn `UserConstructionScript`
  (`/Game/BluePrints/ObjetoBasico/AC_MainObjeto.fGetVariables` (`self.AC_MainObjeto`)))