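; Terrain generator actor that spawns a flat grid of small BP_CubitoVerde cubes on BeginPlay.
; Each cell samples a multi-octave noise function using a random seed and per-sample jitter, built on a sine/cosine stand-in for Perlin noise.
; The octave loop reuses the same coordinates, varying only amplitude.
; The scaled noise selects among three height bands, but all branches currently spawn the same cube at zero height.
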(event `self.ReceiveBeginPlay`
  (set `self.mSeed` (`KismetMathLibrary.RandomFloatInRange` 0.0 100000.0))
  (for _index (range (`self.mGridSizeX`))
    (for _index_2 (range (`self.mGridSizeY`))
      (bind _mhigh (`self.F Multi Octave Perlin Noise 2D` (+ (* _index (`self.mPerlinScale`)) (+ (`self.mSeed`) (`KismetMathLibrary.RandomFloatInRange` 0.0 3.0))) (+ (* _index_2 (`self.mPerlinScale`)) (+ (`self.mSeed`) (`KismetMathLibrary.RandomFloatInRange` 0.0 3.0)))))
      (bind _returnvalue (`KismetMathLibrary.FTrunc` (* (/ (+ _mhigh 1.0) 2.0) (`self.mHeightMultiplier`))))
      (if (< _returnvalue 2)
        (bind _returnvalue_2 (`KismetMathLibrary.MakeTransform` (`KismetMathLibrary.MakeVector` (* _index 10.0) (* _index_2 10.0)) (struct) (0.1 0.1 0.1)))
        (`|SpawnActorFromClass` "/Game/BluePrints/Mundo/BP_CubitoVerde.BP_CubitoVerde_C" _returnvalue_2 "Undefined" "MultiplyWithRoot" null null)
        (elif (> _returnvalue 4)
          (`|SpawnActorFromClass` "/Game/BluePrints/Mundo/BP_CubitoVerde.BP_CubitoVerde_C" _returnvalue_2 "Undefined" "MultiplyWithRoot" null null)
          (else
            (`|SpawnActorFromClass` "/Game/BluePrints/Mundo/BP_CubitoVerde.BP_CubitoVerde_C" _returnvalue_2 "Undefined" "MultiplyWithRoot" null null)))))))

(fn `F Multi Octave Perlin Noise 2D`
  (params (PosX :type "Float (double-precision)") (PosY :type "Float (double-precision)"))
  (returns (mHigh :type "Float (double-precision)"))
  (locals (Total :type "Float (double-precision)") (MaxValue :type "Float (double-precision)") (Frequency :type "Float (double-precision)") (Amplitude :type "Float (double-precision)") (CurrentPosX :type "Float (double-precision)") (CurrentPosY :type "Float (double-precision)"))
  (set `local.CurrentPosX` PosX)
  (set `local.CurrentPosY` PosY)
  (set `local.Frequency` (`self.InitialFrequency`))
  (set `local.Amplitude` (`self.InitialAmplitude`))
  (set `local.CurrentPosX` (* (`local.CurrentPosX`) (`local.Frequency`)))
  (set `local.CurrentPosY` (* (`local.CurrentPosY`) (`local.Frequency`)))
  (set `local.MaxValue` 0.0)
  (for _ (range (`self.Octaves`))
    (bind _mhigh (`self.fOwnPerlin` (`local.CurrentPosX`) (`local.CurrentPosY`)))
    (set `local.MaxValue` (+ (`local.MaxValue`) (`local.Amplitude`)))
    (set `local.Total` (+ (* _mhigh (`local.Amplitude`)) (`local.Total`)))
    (set `local.Frequency` (* (`local.Frequency`) (`self.Lacunarity`)))
    (bind _output_get (set `local.Amplitude` (* (`local.Amplitude`) (`self.Persistence`))))
    (set `local.Total` (+ _output_get (`local.Total`))))
  (bind _output_get_2 (set `local.Total` (/ (`local.Total`) (`local.MaxValue`))))
  (return _output_get_2))

(fn `fOwnPerlin`
  (params (mPosX :type "Float (double-precision)") (mPosY :type "Float (double-precision)"))
  (returns (mHigh :type "Float (double-precision)"))
  (locals (mFrequency :type "Float (double-precision)" :default 10.0))
  (return (/ (+ (`KismetMathLibrary.DegSin` (* mPosX (`local.mFrequency`))) (`KismetMathLibrary.DegCos` (* mPosY (`local.mFrequency`)))) 2.0)))

(fn `UserConstructionScript`)