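; Spawner actor that populates an RTS-style map with trees, gold, berries, a town center and starting villagers.
; FSpawnPlayer, not called within this Blueprint, spawns configurable resource counts at random positions, then the town center with villagers at the same point.
; FGetPositionToSpawn recursively retries positions found in MResourcePositionsList, but never records new ones, and its pure random nodes re-roll between check and return.
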(fn `fGetPositionToSpawn`
  (params (High :type "Float (double-precision)"))
  (returns (NewParam :type "Vector Structure"))
  (bind _returnvalue (`KismetMathLibrary.MakeVector` (`KismetMathLibrary.Conv_IntToDouble` (`KismetMathLibrary.RandomIntegerInRange` 5 2994)) (`KismetMathLibrary.Conv_IntToDouble` (`KismetMathLibrary.RandomIntegerInRange` 5 2994)) High))
  (if (`KismetArrayLibrary.Array_Contains` (`self.mResourcePositionsList`) _returnvalue)
    (bind _newparam (`self.fGetPositionToSpawn` High))
    (return _newparam)
    (else
      (return _returnvalue))))

(fn `fSpawnPlayer`
  (for _ (range (+ (`self.mNumberOfTrees`) 1))
    (bind _newparam (`self.fGetPositionToSpawn` 90.0))
    (`|SpawnActorFromClass` "/Game/BluePrints/Mundo/Resources/BP_Tree.BP_Tree_C" (`KismetMathLibrary.MakeTransform` _newparam (struct) (0.3 0.3 0.3)) "AdjustIfPossibleButAlwaysSpawn" "MultiplyWithRoot" null null))
  (for _ (range (+ (`self.mNumberOfGold`) 1))
    (bind _newparam_2 (`self.fGetPositionToSpawn` 100.0))
    (`|SpawnActorFromClass` "/Game/BluePrints/Mundo/Resources/BP_Gold.BP_Gold_C" (`KismetMathLibrary.MakeTransform` _newparam_2 (struct) (0.1 0.1 0.1)) "AdjustIfPossibleButAlwaysSpawn" "MultiplyWithRoot" null null))
  (for _ (range (+ (`self.mNumberOfBayas`) 1))
    (bind _newparam_3 (`self.fGetPositionToSpawn` 100.0))
    (`|SpawnActorFromClass` "/Game/BluePrints/Mundo/Resources/BP_Berry.BP_Berry_C" (`KismetMathLibrary.MakeTransform` _newparam_3 (struct) (0.5 0.5 0.5)) "AdjustIfPossibleButAlwaysSpawn" "MultiplyWithRoot" null null))
  (bind _newparam_4 (`self.fGetPositionToSpawn` 120.0))
  (`|SpawnActorFromClass` "/Game/BluePrints/Mundo/Buildings/BP_TownCenter.BP_TownCenter_C" (`KismetMathLibrary.MakeTransform` _newparam_4 (struct) (0.2 0.2 0.4)) "AdjustIfPossibleButAlwaysSpawn" "MultiplyWithRoot" null null)
  (for _ (range 3)
    (`|SpawnActorFromClass` "/Game/BluePrints/Personajes/BP_Villager.BP_Villager_C" (`KismetMathLibrary.MakeTransform` _newparam_4 (struct) (0.3 0.3 0.3)) "AdjustIfPossibleButAlwaysSpawn" "MultiplyWithRoot" null null)))

(fn `UserConstructionScript`)